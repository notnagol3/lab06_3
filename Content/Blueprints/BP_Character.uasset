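; First-person character Blueprint with mouse look and strafing; forward movement input is left disconnected.
; Every tick, a debug-drawn visibility line trace from the camera stores any hit actor implementing BP_interact_interface as the current interact target.
; A mouse click sends InteractMessage to that target, or otherwise teleports the character to the trace's hit location, giving gaze-based interaction and movement.
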(event Custom|GazeCheck
  (bind _camera (Variables|Default|GetCamera))
  (bind _returnvalue (Transformation|GetWorldLocation _camera))
  ;[1 1 1] Gaze check
  (bind _outhit (Collision|LineTraceByChannel _returnvalue (+ _returnvalue (* (Math|Vector|GetForwardVector _camera) 2000)) "TraceTypeQuery1" false 0 "ForOneFrame"))
  (if (Utilities|DoesObjectImplementInterface (.HitActor (Collision|BreakHitResult _outhit)) "/Game/Blueprints/BP_interact_interface.BP_interact_interface_C")
    (Variables|Default|Setinteract (.HitActor (Collision|BreakHitResult _outhit)))
    (else
      (Variables|Default|Setinteract 0))))

(event EventTick
  (params (DeltaSeconds :type Float%20%28single-precision%29))
  (CallFunction|GazeCheck))

(event Input|ActionEvents|InputActionmouseclick
  (params (Key :type Key%20Structure :default "None"))
  (bind _interact (Variables|Default|Getinteract))
  (:Pressed
    ;[1 1 1] Input
    (Utilities|IsValid _interact
      (:Is%20Valid
        (Class|BPInteractInterface|Interact(Message) _interact))
      (:Is%20Not%20Valid
        (Transformation|Teleport (.Location (Collision|BreakHitResult (stale Custom|GazeCheck _outhit))) "0, 0, 0")))))

(event Input|AxisEvents|InputAxismouseX
  (params (AxisValue :type Float%20%28single-precision%29))
  ;[1 1 1] Input
  (Pawn|Input|AddControllerYawInput AxisValue))

(event Input|AxisEvents|InputAxismouseY
  (params (AxisValue :type Float%20%28single-precision%29))
  ;[1 1 1] Input
  (Pawn|Input|AddControllerPitchInput AxisValue))

(event Input|AxisEvents|InputAxismoveLeftRight
  (params (AxisValue :type Float%20%28single-precision%29))
  ;[1 1 1] Input
  (Pawn|Input|AddMovementInput (Transformation|GetActorRightVector) AxisValue false))

(event Input|AxisEvents|InputAxismoveForward
  (params (AxisValue :type Float%20%28single-precision%29))
  (if true
    _))

(fn ConstructionScript)